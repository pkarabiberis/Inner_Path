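; Ego is a side-scrolling flipbook character that runs, jumps, throws kunai and dies.
; Tick selects animation from transformed, dead, throwing and movement states, flags death at zero HP, and stops once transformed.
; The egoThrow event spawns a kunai at an arrow component, using delays and a DoOnce gate.
; Stamina-based sword damage against Knight, Rabbit and Scorpio, plus its overlap detection, is disconnected and never runs.
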(event `InputAction|Sword`
  (params (Key :type "Key Structure")))

(event `self.Box.OnComponentBeginOverlap`
  (params (OverlappedComponent :type "PrimitiveComponent Object Reference") (OtherActor :type "Actor Object Reference") (OtherComp :type "PrimitiveComponent Object Reference") (OtherBodyIndex :type Integer) (bFromSweep :type Boolean) (SweepResult :type "HitResult Structure (by ref)")))

(event `UpdateAnimation`
  ;[1 1 1] Handle Animation
  (if (`NavMovementComponent.IsFalling` (`self.CharacterMovement`))
    (`/Engine/EditorBlueprintResources/StandardMacros.DoOnce` false :!label _label
      (:`Completed`
        (`PaperFlipbookComponent.SetFlipbook` (`self.Sprite`) "/Game/test/Monk/Anim/Monk_Jump.Monk_Jump")
        (`KismetSystemLibrary.Delay` 0.44)
        (`PaperFlipbookComponent.SetFlipbook` (`self.Sprite`) "/Game/test/Monk/Monk_jump3.Monk_jump3")))
    (elif (> (`KismetMathLibrary.VSize` (`self.GetVelocity`)) 0.0)
      (`PaperFlipbookComponent.SetFlipbook` (`self.Sprite`) "/Game/Actors/Ego/Flipbooks/Run/Ego_run.Ego_run")
      (else
        (`PaperFlipbookComponent.SetFlipbook` (`self.Sprite`) "/Game/Actors/Ego/Sprites/Ego_idle.Ego_idle")))))

(event `self.OnLanded`
  (params (Hit :type "HitResult Structure (by ref)"))
  ;[1 1 1] Handle Animation
  (goto _label :!via `Reset`))

(event `self.ReceiveBeginPlay`
  (`ActorComponent.SetIsReplicated` (`self.Sprite`) true))

(event `atkthrow`
  ;[1 1 1] Handle Animation
  (if (`NavMovementComponent.IsFalling` (`self.CharacterMovement`))
    (`PaperFlipbookComponent.SetFlipbook` (`self.Sprite`) "/Game/Actors/Ego/Flipbooks/Throw/Ego_throw.Ego_throw")
    (`KismetSystemLibrary.Delay` 0.2)
    (`PaperFlipbookComponent.SetFlipbook` (`self.Sprite`) "/Game/test/Monk/Monk_jump3.Monk_jump3")
    (else
      (`PaperFlipbookComponent.SetFlipbook` (`self.Sprite`) "/Game/Actors/Ego/Flipbooks/Throw/Ego_throw.Ego_throw")
      (`MovementComponent.StopMovementImmediately` (`self.CharacterMovement`)))))

(event `self.Box.OnComponentEndOverlap`
  (params (OverlappedComponent :type "PrimitiveComponent Object Reference") (OtherActor :type "Actor Object Reference") (OtherComp :type "PrimitiveComponent Object Reference") (OtherBodyIndex :type Integer)))

(event `egoThrow`
  ;[1 1 1] Throw
  (`/Engine/EditorBlueprintResources/StandardMacros.DoOnce` false :!label _label_2
    (:`Completed`
      (set `self.Throwing` true)
      (`KismetSystemLibrary.Delay` 0.2)
      (`|SpawnActorFromClass` "/Game/Items/Kunai/Ego_kunai.Ego_kunai_C" (`SceneComponent.K2_GetComponentToWorld` (`self.Arrow1`)) "Undefined" "OverrideRootScale" null null)
      (`KismetSystemLibrary.Delay` 0.2)
      (set `self.Throwing` false)
      (goto _label_2 :!via `Reset`))))

(event `InputAxis|MoveRight`
  (params (AxisValue :type "Float (single-precision)"))
  (bind _returnvalue (`self.GetController`))
  (bind _returnvalue_2 (`self.GetController`))
  ;[1 1 1] Handle movement
  (if (> AxisValue 0.0)
    (set `self.bisMovingRight` true)
    (`/Engine/EditorBlueprintResources/StandardMacros.IsValid` _returnvalue_2
      (:`Is Valid`
        (`Controller.SetControlRotation` _returnvalue_2 (`KismetMathLibrary.MakeRotator` 0.0))))
    (elif (< AxisValue 0.0)
      (set `self.bisMovingRight` false)
      (`/Engine/EditorBlueprintResources/StandardMacros.IsValid` _returnvalue
        (:`Is Valid`
          (`Controller.SetControlRotation` _returnvalue (`KismetMathLibrary.MakeRotator` 0.0 0.0 180.0))))))
  (`self.AddMovementInput` (1.0 0.0 0.0) AxisValue))

(event `self.ReceiveTick`
  (params (DeltaSeconds :type "Float (single-precision)"))
  (bind _sprite (`self.Sprite`))
  ;[1 1 1] Tick - Updates animation
  (if (`self.isTransformed`)
    (`PaperFlipbookComponent.SetFlipbook` _sprite "/Game/test/Monk/Monk_idle_start.Monk_idle_start")
    (`PaperFlipbookComponent.SetSpriteColor` _sprite (struct :`R` 0.005208 :`G` 0.76728 :`B` 1.0 :`A` 1.0))
    (`self.SetActorTickEnabled` false)
    (elif (`self.Dead`)
      (`/Engine/EditorBlueprintResources/StandardMacros.DoOnce` false
        (:`Completed`
          (`PaperFlipbookComponent.SetFlipbook` (`self.Sprite`) "/Game/Actors/Ego/Sprites/EGO_DEATH_FIXED.EGO_DEATH_FIXED")
          (`CharacterMovementComponent.DisableMovement` (`self.CharacterMovement`))
          (`KismetSystemLibrary.Delay` 1.3)
          (`PaperFlipbookComponent.SetFlipbook` (`self.Sprite`) "/Game/Actors/Ego/Sprites/STAYDEADEGO.STAYDEADEGO")))
      (elif (`self.Throwing`)
        (`self.atkthrow`)
        (else
          (`self.UpdateAnimation`)
          (if (<= (`self.HP`) 0.0)
            (set `self.Dead` true)
            (`AddComponent|NODE_AddAudioComponent-1`)))))))

(fn `ResetDodge`
  (set `self.Dodge` true))

(fn `UserConstructionScript`)