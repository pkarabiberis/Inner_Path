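; Checkpoint actor that saves the Monkey's respawn point for Level 01 when the player reaches it.
; When the Monkey's capsule overlaps its Box, it loads the existing checkpoint save game or creates a new one.
; It stores a transform 100 units above the checkpoint with default rotation, sets the transformed and info-HUD-shown flags, then writes the save back to the slot.
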(event `self.ReceiveBeginPlay`)

(event `self.Box.OnComponentBeginOverlap`
  (params (OverlappedComponent :type "PrimitiveComponent Object Reference") (OtherActor :type "Actor Object Reference") (OtherComp :type "PrimitiveComponent Object Reference") (OtherBodyIndex :type Integer) (bFromSweep :type Boolean) (SweepResult :type "HitResult Structure (by ref)"))
  (bind _returnvalue_location (`KismetMathLibrary.BreakTransform` (`self.GetTransform`)))
  (bind _savegameref (`self.SaveGameRef`))
  (bind _asmonkey (cast `/Game/Actors/Monkey/Monkey` OtherActor))
  (if (== OtherComp (`Character.CapsuleComponent` _asmonkey))
    (bind _returnvalue (`GameplayStatics.DoesSaveGameExist` (`self.CheckpointSaveName`)))
    (if _returnvalue
      (bind _returnvalue_2 (`GameplayStatics.LoadGameFromSlot` (`self.CheckpointSaveName`)))
      (bind _ascheckpoint_save_game (cast `/Game/Checkpoint/CheckpointSaveGame` _returnvalue_2))
      (set `self.SaveGameRef` _ascheckpoint_save_game)
      (else
        (bind _returnvalue_3 (`GameplayStatics.CreateSaveGameObject` "/Game/Checkpoint/CheckpointSaveGame.CheckpointSaveGame_C"))
        (set `self.SaveGameRef` _returnvalue_3)))
    (set `/Game/Checkpoint/CheckpointSaveGame.CheckpointLevel01` (`KismetMathLibrary.MakeTransform` (+ _returnvalue_location (0.0 0.0 100.0))) _savegameref)
    (set `/Game/Checkpoint/CheckpointSaveGame.isTransormed` true _savegameref)
    (set `/Game/Checkpoint/CheckpointSaveGame.infoHudShown` true _savegameref)
    (`GameplayStatics.SaveGameToSlot` (`self.SaveGameRef`) (`self.CheckpointSaveName`))))

(fn `UserConstructionScript`)